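; Numbered door Blueprint that serves as the answer check in a room-finding minigame.
; Its construction script applies the chosen door mesh and plate material, then writes the room number as text scaled to the door's width.
; When sent a room number, it tells the game mode to show the end-minigame message on a match, otherwise the cached HUD shows a wrong-room message.
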(event `self.ReceiveBeginPlay`
  (`self.Create_HUD_Ref`))

(event `/Game/Interfaces/BPI_Minigame.Send_Room_Number`
  (params (Room_Number_To_Find :type String))
  (if (== Room_Number_To_Find (`self.Room_Number`))
    (message `/Game/Interfaces/BPI_Minigame.End_Minigame` (`GameplayStatics.GetGameMode`))
    (else
      (message `/Game/Interfaces/BPI_Minigame.Message-Wrong_Room` (`self.HUD-Ref`)))))

(fn `Create_HUD_Ref`
  (bind _asui_hud (cast `/Game/Widgets/UI_HUD` (`PlayerController.GetHUD` (`GameplayStatics.GetPlayerController` 0))))
  (set `self.HUD-Ref` _asui_hud))

(fn `Receive_Minigame_Status`
  (returns (Minigame_Status :type Boolean))
  (return false))

(fn `Receive_Room_Number`
  (returns (Room_Number_To_Find :type String))
  (return ""))

(fn `Receive_Widget_Anim`
  (returns (Anim_1 :type "WidgetAnimation Object Reference") (Anim_2 :type "WidgetAnimation Object Reference"))
  (return null null))

(fn `Setting_Text_Parameters`
  (bind _text_room_number (`self.Text-Room_Number`))
  (bind _returnvalue_x (`KismetMathLibrary.BreakVector` (`SceneComponent.K2_GetComponentScale` (`self.Door`))))
  ;[0.7552 0.1809 0.6881 0.75 22] Setting Parameters Of Text-Room_Number
  ;;[0 0.7656 0.6828 0.75] Changing Content Of The Text
  (`TextRenderComponent.K2_SetText` _text_room_number (`KismetTextLibrary.Conv_StringToText` (`self.Room_Number`)))
  ;;[0.07812 0.8333 0.3443 0.75] Making Text Adjust To The Size Of Door
  (`SceneComponent.SetWorldScale3D` _text_room_number (`KismetMathLibrary.MakeVector` 1.0 _returnvalue_x 1.0)))

(fn `UserConstructionScript`
  (`|ExecutionSequence`
    (:`then_0`
      ;[0.8646 0.7116 0.08106 0.75] Choosing Door Model
      (`StaticMeshComponent.SetStaticMesh` (`self.Door`) (`self.Door_Mesh`)))
    (:`then_1`
      (`self.Setting_Text_Parameters`))
    (:`then_2`
      (`PrimitiveComponent.SetMaterial` (`self.Plate`) 0 (`self.M_Plate`)))))