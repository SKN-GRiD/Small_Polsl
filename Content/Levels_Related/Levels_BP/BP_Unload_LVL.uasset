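; Trigger actor that unloads a configured list of streamed levels when anything overlaps its LoadUnload_LVLs component.
; Overlap resets the index, then a check function caches the Unload array's last index and starts unloading if the array is not empty.
; The unload event loops by calling itself, issuing a non-blocking soft-reference unload and printing a debug string before advancing to the next level.
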(event `self.Load/Unload_LVLs.OnComponentBeginOverlap`
  (params (OverlappedComponent :type "PrimitiveComponent Object Reference") (OtherActor :type "Actor Object Reference") (OtherComp :type "PrimitiveComponent Object Reference") (OtherBodyIndex :type Integer) (bFromSweep :type Boolean) (SweepResult :type "HitResult Structure (by ref)"))
  (set `self.LVL_Index-Current` 0)
  (`self.Decide_If_To_Unload_Streamed_LVLs`))

(event `Unload_LVLs`
  (`GameplayStatics.UnloadStreamLevelBySoftObjectPtr` (`|GetArrayItem` (`self.Unload`) (`self.LVL_Index-Current`)))
  (`KismetSystemLibrary.PrintString` "Unload")
  ;[0.4826 0.0769 0.7031 0.75 22] Unload LVLs - Decision Loop
  (bind _output_get (set `self.LVL_Index-Current` (+ (`self.LVL_Index-Current`) 1)))
  (if (<= _output_get (`self.LV_Index-Max`))
    (`self.Unload_LVLs`)))

(fn `Decide_If_To_Unload_Streamed_LVLs`
  (bind _returnvalue (- (`KismetArrayLibrary.Array_Length` (`self.Unload`)) 1))
  ;[0 0 0 0.75 22] If Array Is Not Empty Start Unloading It's Content
  (set `self.LV_Index-Max` _returnvalue)
  (if (>= _returnvalue 0)
    (`self.Unload_LVLs`)))

(fn `UserConstructionScript`)