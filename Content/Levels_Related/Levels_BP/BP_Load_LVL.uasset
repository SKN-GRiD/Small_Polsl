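; Level streaming trigger that loads a list of sublevels when its Load_LVL collision component is overlapped.
; The overlap resets the index and checks that the Load array has entries before starting.
; A self-calling event then streams each soft-referenced level in sequence without blocking, making it visible and advancing until the last entry.
; The overlap has no actor filter or one-time guard.
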(event `self.Load_LVL.OnComponentBeginOverlap`
  (params (OverlappedComponent :type "PrimitiveComponent Object Reference") (OtherActor :type "Actor Object Reference") (OtherComp :type "PrimitiveComponent Object Reference") (OtherBodyIndex :type Integer) (bFromSweep :type Boolean) (SweepResult :type "HitResult Structure (by ref)"))
  (set `self.LVL_Index-Current` 0)
  (`self.Decide_If_To_Load_Streamed_LVLs`))

(event `Load_LVLs`
  ;[0.8646 0.04503 0.6157 0.75 22] Load LVLs
  (`GameplayStatics.LoadStreamLevelBySoftObjectPtr` (`|GetArrayItem` (`self.Load`) (`self.LVL_Index-Current`)) true)
  ;;[0.0769 0.09869 0.7031 0.75 22] Load LVLs - Decision Loop
  (bind _output_get (set `self.LVL_Index-Current` (+ (`self.LVL_Index-Current`) 1)))
  (if (<= _output_get (`self.LV_Index-Max`))
    (`self.Load_LVLs`)))

(fn `Decide_If_To_Load_Streamed_LVLs`
  (bind _returnvalue (- (`KismetArrayLibrary.Array_Length` (`self.Load`)) 1))
  ;[0.5 0.5 0.5 0.75 22] If Array Is Not Empty Start Loading It's Content
  (set `self.LV_Index-Max` _returnvalue)
  (if (>= _returnvalue 0)
    (`self.Load_LVLs`)))

(fn `UserConstructionScript`)