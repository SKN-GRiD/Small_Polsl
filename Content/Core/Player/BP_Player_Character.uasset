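; Player character Blueprint that handles movement, camera look, UI toggles and minigame interaction.
; BeginPlay registers the Enhanced Input mapping, caches the UI_HUD and enables its gameplay overlay.
; Map and menu inputs flip-flop HUD screens, with the map toggle blocked while the menu is in the viewport.
; When the GameMode's minigame status allows, interaction box-traces around the mesh and sends the GameMode's room number to the hit actor.
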(event `self.ReceiveBeginPlay`
  (`|ExecutionSequence`
    (:`then_0`
      (`self.Appending_Input_System`))
    (:`then_1`
      (`self.Create_HUD_Ref`))
    (:`then_2`
      (`/Game/Widgets/UI_HUD.Enable_Gameplay_Overlay` (`self.HUD_Ref`)))))

(event `EnhancedInput|/Game/Core/Input/IA_Move_Forward-Backward`
  (params (ActionValue :type "Float (double-precision)") (ElapsedSeconds :type "Float (double-precision)") (TriggeredSeconds :type "Float (double-precision)") (InputAction :type "InputAction Object Reference" :default "/Game/Core/Input/IA_Move_Forward-Backward.IA_Move_Forward-Backward"))
  (bind (_returnvalue_roll _returnvalue_pitch _returnvalue_yaw) (`KismetMathLibrary.BreakRotator` (`self.GetControlRotation`)))
  ;[0.5781 0.0368 0.225 0.75 22] Movement System
  ;;[0 0.5521 0.1727 0.75 22] Forward-Backward Movement
  (:`Triggered`
    (`self.AddMovementInput` (`KismetMathLibrary.GetForwardVector` (`KismetMathLibrary.MakeRotator` 0.0 0.0 _returnvalue_yaw)) (* ActionValue (`self.Movement_Speed`)))))

(event `EnhancedInput|/Game/Core/Input/IA_Move_Left-Right`
  (params (ActionValue :type "Float (double-precision)") (ElapsedSeconds :type "Float (double-precision)") (TriggeredSeconds :type "Float (double-precision)") (InputAction :type "InputAction Object Reference" :default "/Game/Core/Input/IA_Move_Left-Right.IA_Move_Left-Right"))
  (bind (_returnvalue_roll _returnvalue_pitch _returnvalue_yaw) (`KismetMathLibrary.BreakRotator` (`self.GetControlRotation`)))
  ;[0.5781 0.0368 0.225 0.75 22] Movement System
  ;;[0 0.8177 0.01314 0.75 22] Left-Right Movement
  (:`Triggered`
    (`self.AddMovementInput` (`KismetMathLibrary.GetRightVector` (`KismetMathLibrary.MakeRotator` 0.0 0.0 _returnvalue_yaw)) (* ActionValue (`self.Movement_Speed`)))))

(event `EnhancedInput|/Game/Core/Input/IA_Look_Around`
  (params (ActionValue :type "Vector2D Structure") (ElapsedSeconds :type "Float (double-precision)") (TriggeredSeconds :type "Float (double-precision)") (InputAction :type "InputAction Object Reference" :default "/Game/Core/Input/IA_Look_Around.IA_Look_Around"))
  ;[0.08854 1 0.3021 0.5 24] Camera
  (:`Triggered`
    (`self.AddControllerYawInput` ActionValue_X)
    (`self.AddControllerPitchInput` ActionValue_Y)))

(event `EnhancedInput|/Game/Core/Input/IA_Enable_Map`
  (params (ActionValue :type "Float (double-precision)") (ElapsedSeconds :type "Float (double-precision)") (TriggeredSeconds :type "Float (double-precision)") (InputAction :type "InputAction Object Reference" :default "/Game/Core/Input/IA_Enable_Map.IA_Enable_Map"))
  ;[0.7708 0.5781 0 0.75 22] Map Widget Interaction
  (:`Started`
    (`self.is_UI_Menu_On`
      (:`Output`
        (`/Engine/EditorBlueprintResources/StandardMacros.FlipFlop`
          (:`A`
            (`/Game/Widgets/UI_HUD.Enable_Map` (`self.HUD_Ref`)))
          (:`B`
            (`/Game/Widgets/UI_HUD.Disable_Map` (`self.HUD_Ref`))))))))

(event `EnhancedInput|/Game/Core/Input/IA_Enable_Menu`
  (params (ActionValue :type "Float (double-precision)") (ElapsedSeconds :type "Float (double-precision)") (TriggeredSeconds :type "Float (double-precision)") (InputAction :type "InputAction Object Reference" :default "/Game/Core/Input/IA_Enable_Menu.IA_Enable_Menu"))
  (:`Started`
    (`/Engine/EditorBlueprintResources/StandardMacros.FlipFlop`
      (:`A`
        (`/Game/Widgets/UI_HUD.Enable_Menu` (`self.HUD_Ref`)))
      (:`B`
        (`/Game/Widgets/UI_HUD.Disable_Menu` (`self.HUD_Ref`))))))

(event `EnhancedInput|/Game/Core/Input/IA_Minigame_Interaction`
  (params (ActionValue :type "Float (double-precision)") (ElapsedSeconds :type "Float (double-precision)") (TriggeredSeconds :type "Float (double-precision)") (InputAction :type "InputAction Object Reference" :default "/Game/Core/Input/IA_Minigame_Interaction.IA_Minigame_Interaction"))
  ;[0.7812 0.08263 0.5963 0.5 22] Minigame
  (:`Started`
    (bind _minigame_status (message `/Game/Interfaces/BPI_Minigame.Receive_Minigame_Status` (`GameplayStatics.GetGameMode`)))
    (if _minigame_status
      (bind _outhit_hitactor (`self.Room_Detection_Box`))
      (bind _room_number_to_find (message `/Game/Interfaces/BPI_Minigame.Receive_Room_Number` (`GameplayStatics.GetGameMode`)))
      (message `/Game/Interfaces/BPI_Minigame.Send_Room_Number` _outhit_hitactor _room_number_to_find))))

(fn `Appending_Input_System`
  (bind _returnvalue (pcsubsystem `EnhancedInputLocalPlayerSubsystem` (`GameplayStatics.GetPlayerController` 0)))
  (`/Engine/EditorBlueprintResources/StandardMacros.IsValid` _returnvalue
    (:`Is Valid`
      (`EnhancedInputSubsystemInterface.AddMappingContext` _returnvalue "/Game/Core/Input/IM_Movement.IM_Movement" 0 (struct))
      (`EnhancedInputUserSettings.RegisterInputMappingContext` (`EnhancedInputSubsystemInterface.GetUserSettings` _returnvalue) "/Game/Core/Input/IM_Movement.IM_Movement"))))

(fn `Create_HUD_Ref`
  (bind _asui_hud (cast `/Game/Widgets/UI_HUD` (`PlayerController.GetHUD` (`GameplayStatics.GetPlayerController` 0))))
  (set `self.HUD_Ref` _asui_hud))

(fn `Room_Detection_Box`
  (returns (OutHit_HitActor :type "Actor Object Reference"))
  (bind _mesh (`self.Mesh`))
  (bind (_returnvalue_roll _returnvalue_pitch _returnvalue_yaw) (`KismetMathLibrary.BreakRotator` (`SceneComponent.K2_GetComponentRotation` _mesh)))
  (bind _returnvalue (`SceneComponent.K2_GetComponentLocation` _mesh))
  (bind _outhit (`KismetSystemLibrary.BoxTraceSingle` :`Start` (+ _returnvalue (0.0 0.0 100.0)) :`End` (- _returnvalue (0.0 0.0 50.0)) :`HalfSize` (200.0 100.0 0.0) :`Orientation` (`KismetMathLibrary.MakeRotator` 0.0 0.0 _returnvalue_yaw) :`TraceChannel` "TraceTypeQuery3" :`DrawDebugType` "ForDuration" :`DrawTime` 2.0))
  (return (`.HitActor` (`GameplayStatics.BreakHitResult` _outhit))))

(fn `UserConstructionScript`)