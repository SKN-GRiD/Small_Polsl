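; Game mode that runs the "Find_Room" minigame and applies fixed graphics settings (anti-aliasing, VSync, frame cap) at BeginPlay.
; Starting the minigame picks a random row from the selected floor's data table, stores its room number and turns on the HUD's minigame messages.
; Ending it clears the active flag and shows the HUD's end message through the cached UI_HUD reference.
; Getter functions expose the active state and room number.
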(event `self.ReceiveBeginPlay`
  (`|ExecutionSequence`
    (:`then_0`
      ;[0.8542 0.2674 0 0.5 22] Create Refrence To UI_HUD
      (bind _asui_hud (cast `/Game/Widgets/UI_HUD` (`PlayerController.GetHUD` (`GameplayStatics.GetPlayerController` 0))))
      (set `self.UI_HUD_Ref` _asui_hud))
    (:`then_1`
      (`self.Settings`))))

(event `/Game/Interfaces/BPI_Minigame.Start_Minigame`
  (params (Floor_Number_To_Select_From :type Integer))
  ;[0.0274 0.01626 0.5885 0.5 22] Start Minigame "Find_Room"
  (set `self.Is_Minigame_Active` true)
  (`self.Choose_Random_Room_Number` Floor_Number_To_Select_From))

(event `/Game/Interfaces/BPI_Minigame.End_Minigame`
  ;[0.6562 0.00034 0.09244 0.75 22] End Minigame "Find_Room"
  (set `self.Is_Minigame_Active` false)
  (message `/Game/Interfaces/BPI_Minigame.End_Minigame` (`self.UI_HUD_Ref`)))

(fn `Receive_Minigame_Status`
  (returns (Minigame_Status :type Boolean))
  (return (`self.Is_Minigame_Active`)))

(fn `Receive_Room_Number`
  (returns (Room_Number_To_Find :type String))
  (return (`self. Room_Number`)))

(fn `Receive_Widget_Anim`
  (returns (Anim_1 :type "WidgetAnimation Object Reference") (Anim_2 :type "WidgetAnimation Object Reference"))
  (return null null))

(fn `Settings`
  (bind _returnvalue (`GameUserSettings.GetGameUserSettings`))
  (`GameUserSettings.SetAntiAliasingQuality` _returnvalue 3)
  (`GameUserSettings.SetVSyncEnabled` _returnvalue true)
  (`GameUserSettings.SetFrameRateLimit` _returnvalue 90.0))

(fn `UserConstructionScript`)